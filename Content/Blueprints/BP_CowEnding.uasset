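; BP_CowEnding is a cow actor, apparently for the game's ending, that can be blown up or hidden on demand.
; Blowup plays an explosion sound at the actor's location and applies a strong impulse to its static mesh, with a fixed upward force and randomized, non-negative X and Y components.
; Disappear hides the actor in game without destroying it.
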(fn `Blowup`
  ;[1 1 1] Get location
  (`GameplayStatics.PlaySoundAtLocation` "/Game/StarterContent/Audio/Explosion_Cue.Explosion_Cue" (`KismetMathLibrary.TransformLocation` (`self.GetTransform` self)) (struct) 1.0 1.0 0.0 null null null null)
  (`PrimitiveComponent.AddImpulse` (`self.StaticMeshComponent`) (`KismetMathLibrary.MakeVector` (`KismetMathLibrary.RandomFloatInRange` 0.0 200000.0) (`KismetMathLibrary.RandomFloatInRange` 0.0 200000.0) 200000.0) "None" false))

(fn `Disappear`
  (`self.SetActorHiddenInGame` true))

(fn `UserConstructionScript`)